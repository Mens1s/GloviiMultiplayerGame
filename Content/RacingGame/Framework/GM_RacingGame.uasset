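; Game mode for a timed checkpoint race, where the player must cross the finish line before time runs out.
; BeginPlay binds to every BP_Checkpoint, handling the finish line separately, then runs a start countdown before starting the time-remaining timer.
; Checkpoints restart that timer with added time and play a vehicle HUD animation.
; Winning clears the timer; both win and loss currently only print a result.
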(event `self.ReceiveBeginPlay`
  (`|ExecutionSequence`
    (:`then_0`
      (bind _outactors (`GameplayStatics.GetAllActorsOfClass` "/Game/RacingGame/CheckPoints/BP_Checkpoint.BP_Checkpoint_C" :!pinned true)) ; checkpointleri geitr
      (for _array_element _outactors
        (if (`/Game/RacingGame/CheckPoints/BP_Checkpoint.IsFinishLine` _array_element)
          (add `/Game/RacingGame/CheckPoints/BP_Checkpoint.OnCheckpointCrossed` _array_element (`|CreateDelegate` :!event `Win_CrossTheFinishLine`))
          (else
            (add `/Game/RacingGame/CheckPoints/BP_Checkpoint.OnCheckPointCrossedWithTime` _array_element (`|CreateDelegate` :!event `CrossedACheckpoint`))))))
    (:`then_1`
      (`self.Start Countdown`))))

(event `Start Countdown`
  (`KismetSystemLibrary.PrintString` "Hello")
  (`KismetSystemLibrary.Delay` (`self.StartCountdownDuration`))
  (`self.Game Start`))

(event `Game Start`
  (`KismetSystemLibrary.PrintString` "Hello")
  (bind _returnvalue (`KismetSystemLibrary.K2_SetTimerDelegate` (delegate `Lose_OutOfTime`) (`self.StartTimerDuration`)))
  (set `self.TimeRemainingTimer` _returnvalue))

(event `Lose_OutOfTime`
  (`self.Game Finish` false))

(event `Win_CrossTheFinishLine`
  (`KismetSystemLibrary.K2_ClearAndInvalidateTimerHandle` (`self.TimeRemainingTimer`))
  (`self.Game Finish` true))

(event `Game Finish`
  (params (Win :type Boolean))
  (`KismetSystemLibrary.PrintString` (`KismetMathLibrary.SelectString` "You Win" "You Lost" Win)))

(event `CrossedACheckpoint`
  (params (TimeToAdd :type Integer))
  (`self.AddTimeToTimer` TimeToAdd))

(fn `AddTimeToTimer`
  (params (TimeToAdd :type Integer))
  (bind _returnvalue (`KismetSystemLibrary.K2_SetTimerDelegate` (`|CreateDelegate` :!event `Lose_OutOfTime`) (+ (`local.TimeToAdd`) (`KismetSystemLibrary.K2_GetTimerRemainingTimeHandle` (`self.TimeRemainingTimer`)))))
  (set `self.TimeRemainingTimer` _returnvalue)
  (bind _asvehicle_player_controller (cast `/Game/VehicleTemplate/Blueprints/VehiclePlayerController` (`GameplayStatics.GetPlayerController` 0)))
  (`/Game/VehicleTemplate/Blueprints/VehicleUI.PlayAddedTimeAnimation` (`/Game/VehicleTemplate/Blueprints/VehiclePlayerController.VehicleHud` _asvehicle_player_controller)))

(fn `NewFunction`
  (params (NewParam :type Boolean))
  (returns (NewParam1 :type Boolean))
  (return false))

(fn `UserConstructionScript`)